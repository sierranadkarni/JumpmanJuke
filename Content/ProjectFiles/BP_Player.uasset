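; BP_Player is the player character, handling Enhanced Input movement, jumping, damage and respawn.
; BeginPlay adds the default mapping context after a short delay and passes the spawn transform to GM_DK.
; Movement input runs along the actor's forward vector only.
; Damage sets Health to damage minus current Health, clamped zero to one; at zero the actor destroys itself, and Destroyed asks GM_DK to respawn it.
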(event Input|EnhancedActionEvents|EnhancedInputActionIA_Movement
  (params (ActionValue :type Float%20%28double-precision%29) (ElapsedSeconds :type Float%20%28double-precision%29) (TriggeredSeconds :type Float%20%28double-precision%29) (InputAction :type Input%20Action%20Object%20Reference :default "/Game/ProjectFiles/input/IA_Movement.IA_Movement"))
  ;[1 1 1] Movement
  (Pawn|Input|AddMovementInput (Transformation|GetActorForwardVector) ActionValue false))

(event Input|EnhancedActionEvents|EnhancedInputActionIA_Jump
  (params (ActionValue :type Boolean) (ElapsedSeconds :type Float%20%28double-precision%29) (TriggeredSeconds :type Float%20%28double-precision%29) (InputAction :type Input%20Action%20Object%20Reference :default "/Game/ProjectFiles/input/IA_Jump.IA_Jump"))
  ;[1 1 1] Movement
  (Character|Jump))

(event EventBeginPlay
  ;[1 1 1] Movement
  (Utilities|FlowControl|Delay 0.02)
  (bind _aspc_dk (Utilities|Casting|CastToPC_DK (Game|GetPlayerController 0)))
  (Utilities|IsValid _aspc_dk
    (:Is%20Valid
      (Utilities|IsValid (PlayerController|LocalPlayerSubsystems|GetEnhancedInputLocalPlayerSubsystem _aspc_dk)
        (:Is%20Valid
          (Input|AddMappingContext (PlayerController|LocalPlayerSubsystems|GetEnhancedInputLocalPlayerSubsystem _aspc_dk) "/Game/ProjectFiles/input/IMC_default.IMC_default" 0 "(bIgnoreAllPressedKeysUntilRelease=True,bForceImmediately=False,bNotifyUserSettings=False)")
          (bind _asgm_dk (Utilities|Casting|CastToGM_DK (Game|GetGameMode)))
          (Variables|/Game/ProjectFiles/GM_DK.GM_DK_C|SetRespawn%20Transform _asgm_dk (Variables|Default|GetSpawn)))))))

(event EventDestroyed
  ;[1 1 1] Respawn
  (bind _asgm_dk (Utilities|Casting|CastToGM_DK (Game|GetGameMode)))
  (Default|RespawnPlayer _asgm_dk self))

(event Game|Damage|EventAnyDamage
  (params (Damage :type Float%20%28single-precision%29) (DamageType :type Damage%20Type%20Object%20Reference) (InstigatedBy :type Controller%20Object%20Reference) (DamageCauser :type Actor%20Object%20Reference))
  ;[1 1 1] Damage
  (if (not (Variables|Default|GetIsDead?))
    (bind _output_get (Variables|Default|SetHealth (Math|Float|Clamp(Float) (- Damage (Variables|Default|GetHealth)))))
    (if (== _output_get 0.0)
      (Variables|Default|SetIsDead? true)
      (Actor|DestroyActor))))

(fn ConstructionScript)